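; Player controller that switches the view between a main labyrinth camera and a camel camera, and quits the game on Escape.
; On BeginPlay it blends to the labyrinth camera and slows global time dilation to near standstill.
; Holding CameraSwitching blends to the camel camera; releasing returns to the labyrinth view.
; While held, Tick moves that camera's spring arm above the BP_Camel1 capsule.
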(event Custom|LabyrinthView
  ;[0.06771 0.06771 0.06771] CAMERA SWIRCHING
  ;;[1 1 1] Set LABYRINTH view
  (bind _outactors (Actor|GetAllActorsOfClass "/Game/_BLUEPRINTS/BP_CAMERA_MAIN.BP_CAMERA_MAIN_C"))
  (Variables|Default|SetCamera_Ref (Utilities|Array|Get(acopy) _outactors))
  (Game|Player|SetViewTargetwithBlend (Game|GetPlayerController 0) (Variables|Default|GetCamera_Ref) 0.1 "VTBlend_Linear" 0.0 false))

(event Custom|KamelView
  ;[0.06771 0.06771 0.06771] CAMERA SWIRCHING
  ;;[1 1 1] Set KAMEL view
  (bind _outactors (Actor|GetAllActorsOfClass "/Game/_BLUEPRINTS/BP_CAMERA_KAMEL.BP_CAMERA_KAMEL_C"))
  (Variables|Default|SetCamKAMELref (Utilities|Array|Get(acopy) _outactors))
  (Game|Player|SetViewTargetwithBlend (Game|GetPlayerController 0) (Variables|Default|GetCamKAMELref) 0.1 "VTBlend_Linear" 0.0 false))

(event EventBeginPlay
  ;[1 0.1094 0.1094] EVENT BEGIN PLAY
  (CallFunction|LabyrinthView)
  (Utilities|Time|SetGlobalTimeDilation 0.01))

(event EventTick
  (params (DeltaSeconds :type Float%20%28single-precision%29))
  ;[0.4018 1 0.4524] EVENT TICK - Set cam Kamel location
  (if (Variables|Default|GetKamelCam)
    (bind _outactors (Actor|GetAllActorsOfClass "/Game/_CHARACTER/BP_Camel1.BP_Camel1_C"))
    (for _array_element _outactors
      (Variables|Default|SetCamel_Ref (Variables|/Script/Engine.Character|GetCapsuleComponent _array_element))
      (Transformation|SetWorldLocation (Variables|/Game/_BLUEPRINTS/BP_CAMERA_KAMEL.BP_CAMERA_KAMEL_C|GetSpringArm (Variables|Default|GetCamKAMELref)) (Math|Vector|MakeVector (- (.x (Transformation|GetWorldLocation (Variables|Default|GetCamel_Ref))) 1e+01) (.y (Transformation|GetWorldLocation (Variables|Default|GetCamel_Ref))) (+ (.z (Transformation|GetWorldLocation (Variables|Default|GetCamel_Ref))) 3e+02)) false false))))

(event Input|ActionEvents|InputActionCameraSwitching
  (params (Key :type Key%20Structure :default "None"))
  ;[0.06771 0.06771 0.06771] CAMERA SWIRCHING
  ;;[1 1 1] Camera Switch Input
  (:Pressed
    (Variables|Default|SetKamelCam true)
    (CallFunction|KamelView))
  (:Released
    (Variables|Default|SetKamelCam false)
    (CallFunction|LabyrinthView)))

(event Input|KeyboardEvents|Escape
  (params (Key :type Key%20Structure :default "None"))
  (:Pressed
    (Game|QuitGame 0 "Quit" false)))

(fn ConstructionScript)