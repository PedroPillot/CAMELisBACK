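; Procedural maze actor that builds a seeded, desert-dressed grid maze in its Construction Script using instanced meshes.
; A randomized backtracking carver steps two tiles from a start corner, recording bridge tiles and converting them to paths as it backtracks.
; Leftover tiles become walls, optionally opened into loops.
; Border, floors and walls spawn from index arrays, followed by random cacti and oases on paths and one pineapple near the far corner.
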(event EventBeginPlay)

(event Collision|EventActorBeginOverlap
  (params (OtherActor :type Actor%20Object%20Reference)))

(event EventTick
  (params (DeltaSeconds :type Float%20%28single-precision%29)))

(fn ConstructionScript
  (CallFunction|PopulateBoarders (Variables|Default|GetSize) (Variables|Default|GetBoarderTiles))
  (if (Variables|Default|GetbShowBoarder?)
    (Utilities|SpawnInstances (Variables|Default|GetBoarderTiles) (Variables|Default|GetSize) (Variables|Default|GetTileSize) (Variables|Default|GetMeshScale) (Variables|Default|GetWall)
      (:Finished
        _)))
  (if (Variables|Default|GetbShowMaze?)
    (CallFunction|SetInitialTile)
    (while (Variables|Default|GetbCurrentFreeSide?) :!label _label
      (CallFunction|PickNearbyTile))
    (Utilities|Array|Add (Variables|Default|GetCheckedTiles) (Variables|Default|GetCurrentTile))
    (CallFunction|BackTrack)
    (Utilities|ConvertLastBridge
      (:BridgesLeft
        (goto _label))
      (:NoBridgeLeft
        (CallFunction|PopulateWalls)
        (if (Variables|Default|GetbAllowLoopPaths?)
          (CallFunction|AddLoopPaths))
        (Utilities|SpawnInstances (Variables|Default|GetPathTiles) (Variables|Default|GetSize) (Variables|Default|GetTileSize) "1.000000,1.000000,0.010000" (Variables|Default|GetFloor)
          (:Finished
            (if (Variables|Default|GetbShowWalls?)
              (Utilities|SpawnInstances (Variables|Default|GetWallTiles) (Variables|Default|GetSize) (Variables|Default|GetTileSize) (Variables|Default|GetMeshScale) (Variables|Default|GetWall)
                (:Finished
                  (CallFunction|AddCactus)
                  (Utilities|SpawnInstances (Variables|Default|GetCactusTile) (Variables|Default|GetSize) (Variables|Default|GetTileSize) (* (Variables|Default|GetMeshScale) (Variables|Default|GetTailleCactus)) (Variables|Default|GetCactus)
                    (:Finished
                      (CallFunction|AddOasis)
                      (Utilities|SpawnInstances (Variables|Default|GetOasisTile) (Variables|Default|GetSize) (Variables|Default|GetTileSize) (* (Variables|Default|GetMeshScale) (Variables|Default|GetTailleOasis)) (Variables|Default|GetOasis)
                        (:Finished
                          (CallFunction|AddAnanas)
                          (Utilities|SpawnInstances (Variables|Default|GetAnanasTile) (Variables|Default|GetSize) (Variables|Default|GetTileSize) (* (Variables|Default|GetMeshScale) (Variables|Default|GetTailleOasis)) (Variables|Default|GetAnanas)))))))))))))))

(fn PopulateBoarders
  (params (Size :type Integer) (BoarderArray :type Array%20of%20Integers))
  (LocalVariables|SetL_Size Size)
  ;[1 1 1] North Border
  (for _index (range 0 (- (LocalVariables|GetL_Size) 1))
    (Utilities|Array|Add BoarderArray _index))
  ;[1 1 1] Esat Border
  (for _index_2 (range 1 (- (LocalVariables|GetL_Size) 2))
    (Utilities|Array|Add BoarderArray (+ (* _index_2 (LocalVariables|GetL_Size)) (- (LocalVariables|GetL_Size) 1))))
  ;[1 1 1] South Boarder
  (for _index_3 (range 1 (LocalVariables|GetL_Size))
    (Utilities|Array|Add BoarderArray (+ (- _index_3 1) (* (LocalVariables|GetL_Size) (- (LocalVariables|GetL_Size) 1)))))
  ;[1 1 1] West Boarder
  (for _index_4 (range 1 (- (LocalVariables|GetL_Size) 2))
    (Utilities|Array|Add BoarderArray (* _index_4 (LocalVariables|GetL_Size)))))

(fn SetInitialTile
  (Variables|Default|SetCurrentTile (+ (Variables|Default|GetSize) 1))
  (Utilities|Array|Add (Variables|Default|GetPathTiles) (Variables|Default|GetCurrentTile)))

(fn AddBridge&PathTile
  (params (PathTile :type Integer) (BridgeTile :type Integer))
  (Utilities|Array|Add (Variables|Default|GetPathTiles) PathTile)
  (Variables|Default|SetCurrentTile PathTile)
  (Utilities|Array|Add (Variables|Default|GetBridgeTiles) BridgeTile))

(fn PickNearbyTile
  (bind _currenttile (Variables|Default|GetCurrentTile))
  (bind _size (Variables|Default|GetSize))
  (bind _currenttile_2 (Variables|Default|GetCurrentTile))
  (bind _size_2 (Variables|Default|GetSize))
  (bind _currenttile_3 (Variables|Default|GetCurrentTile))
  (bind _size_3 (Variables|Default|GetSize))
  (bind _currenttile_4 (Variables|Default|GetCurrentTile))
  (bind _size_4 (Variables|Default|GetSize))
  (bind (_btileinarrays_ _pathtile _bridgetile) (Utilities|CheckNorthTile _currenttile_3 _size_3 true))
  (bind (_btileinarrays__2 _pathtile_2 _bridgetile_2) (Utilities|CheckEastTile _currenttile_2 _size_2 true))
  (bind (_btileinarrays__3 _pathtile_3 _bridgetile_3) (Utilities|CheckNorthTile _currenttile_4 _size_4 false))
  (bind (_btileinarrays__4 _pathtile_4 _bridgetile_4) (Utilities|CheckEastTile _currenttile _size false))
  (switch int (Math|Random|RandomIntegerinRangefromStream 0 3 (Variables|Default|GetRandomStream))
    (:0
      (if _btileinarrays__3 :!label _label
        (Utilities|CycleCounter (LocalVariables|GetCycleCount) 4
          (:True
            (if _btileinarrays_ :!label _label_2
              (Utilities|CycleCounter (LocalVariables|GetCycleCount) 4
                (:True
                  (if _btileinarrays__4 :!label _label_3
                    (Utilities|CycleCounter (LocalVariables|GetCycleCount) 4
                      (:True
                        (if _btileinarrays__2 :!label _label_4
                          (Utilities|CycleCounter (LocalVariables|GetCycleCount) 4
                            (:True
                              (goto _label))
                            (:False
                              (Variables|Default|SetbCurrentFreeSide? false :!label _label_5)))
                          (else
                            (CallFunction|AddBridge&PathTile _pathtile_2 _bridgetile_2))))
                      (:False
                        (goto _label_5)))
                    (else
                      (CallFunction|AddBridge&PathTile _pathtile_4 _bridgetile_4))))
                (:False
                  (goto _label_5)))
              (else
                (CallFunction|AddBridge&PathTile _pathtile _bridgetile))))
          (:False
            (goto _label_5)))
        (else
          (CallFunction|AddBridge&PathTile _pathtile_3 _bridgetile_3))))
    (:1
      (goto _label_3))
    (:2
      (goto _label_2))
    (:3
      (goto _label_4)))
  (return))

(fn BackTrack
  (bind _arrayelement (Utilities|ForEachLoopwithBreakRec (Variables|Default|GetPathTiles) :!label _label)
    (:LoopBody
      (if (not (Utilities|Array|ContainsItem (Variables|Default|GetCheckedTiles) _arrayelement))
        (Variables|Default|SetCurrentTile _arrayelement)
        (goto _label Break)))))

(fn PopulateWalls
  (bind _size (Variables|Default|GetSize))
  (for _index (range 0 (- (* _size _size) 1))
    (if (not (Utilities|CheckTileArrays _index))
      (Utilities|Array|Add (Variables|Default|GetWallTiles) _index))))

(fn AddLoopPaths
  (LocalVariables|SetLoopPathsAdded 0)
  (LocalVariables|SetLoopPath (Utilities|GetRandomElement(Array) (Variables|Default|GetWallTiles) (Variables|Default|GetRandomStream)) :!label _label)
  (if (Utilities|TileSurrounded (LocalVariables|GetLoopPath))
    _
    (else
      (Utilities|Add&RemoveItem(Array) (LocalVariables|GetLoopPath) (Variables|Default|GetPathTiles) (Variables|Default|GetWallTiles)
        (:Out
          (LocalVariables|SetLoopPathsAdded (+ (LocalVariables|GetLoopPathsAdded) 1))))))
  (if (< (LocalVariables|GetLoopPathsAdded) (Variables|Default|GetMaxLoopPaths))
    (goto _label)))

(fn AddCactus
  (LocalVariables|SetCactusAdded 0)
  (if (< (LocalVariables|GetCactusAdded) (Variables|Default|GetMaxCactus))
    (bind _output_get (LocalVariables|SetCactusPath (Utilities|GetRandomElement(Array) (Variables|Default|GetPathTiles) (Variables|Default|GetRandomStream)) :!label _label))
    (Utilities|Array|Add (Variables|Default|GetCactusTile) _output_get)
    (LocalVariables|SetCactusAdded (+ (LocalVariables|GetCactusAdded) 1))
    (if (< (LocalVariables|GetCactusAdded) (Variables|Default|GetMaxCactus))
      (goto _label))))

(fn AddOasis
  (LocalVariables|SetOasisAdded 0)
  (if (< (LocalVariables|GetOasisAdded) (Variables|Default|GetMaxOasis))
    (bind _output_get (LocalVariables|SetOasisPath (Utilities|GetRandomElement(Array) (Variables|Default|GetPathTiles) (Variables|Default|GetRandomStream)) :!label _label))
    (Utilities|Array|Add (Variables|Default|GetOasisTile) _output_get)
    (LocalVariables|SetOasisAdded (+ (LocalVariables|GetOasisAdded) 1))
    (if (< (LocalVariables|GetOasisAdded) (Variables|Default|GetMaxOasis))
      (goto _label))))

(fn AddAnanas
  (Utilities|Array|Add (Variables|Default|GetAnanasTile) (- (- (* (Variables|Default|GetSize) (Variables|Default|GetSize)) (* (Variables|Default|GetSize) 1)) 2)))